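; Enemy character for a game jam that patrols PatrolPointBP actors until pawn sensing spots the player, then chases permanently.
; Tick drives AI movement and turns IsKicked into a backward launch with a brief IsKickedinto window.
; Range-finder overlaps during that window cost HP, otherwise briefly halt movement; any overlap advances the patrol index.
; High-MaxHP enemies get a strong material; destruction adds player score and removes the range finder.
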(event OnSeePawn(PawnSensing)
  (params (Pawn :type Pawn%20Object%20Reference))
  (if (Pawn|IsPlayerControlled Pawn)
    (Variables|Default|SetseenPlayer true)))

(event EventBeginPlay
  (Variables|Default|SetHP (Variables|Default|GetmaxHP))
  (if (> (Variables|Default|GetmaxHP) 2.0)
    (Rendering|Material|SetMaterial (Variables|Character|GetMesh) 0 "/Game/GameJam/Material/m_StrongEnemy.m_StrongEnemy")
    (Rendering|Material|SetMaterial (Variables|Character|GetMesh) 1 "/Game/GameJam/Material/m_StrongEnemy.m_StrongEnemy")))

(event Collision|EventActorBeginOverlap
  (params (OtherActor :type Actor%20Object%20Reference))
  (Utilities|FlowControl|Sequence
    (:then_0
      (Utilities|Casting|CastToEnemyRangeFinderBP OtherActor)
      (if (Variables|Default|GetisKickedinto)
        (bind _result (Math|Float|DecrementFloat (Variables|Default|GetHP))
          (:%20%20
            (Variables|Default|SetHP _result)
            (if (<= (Variables|Default|GetHP) 0.0)
              (Actor|DestroyActor))))
        (else
          (Components|Movement|StopMovementImmediately (Variables|Character|GetCharacterMovement))
          (Variables|Default|SetMovement%20prevention true))))
    (:then_1
      (bind _result_2 (Math|Integer|IncrementInt (Variables|Default|GetcurrentNavpoint))
        (:%20%20
          (Variables|Default|SetcurrentNavpoint _result_2)
          (if (not (Utilities|Array|IsValidIndex (Variables|Default|GetPatrolPointBP) (Variables|Default|GetcurrentNavpoint)))
            (Variables|Default|SetcurrentNavpoint 0)))))))

(event EventTick
  (params (DeltaSeconds :type Float%20%28single-precision%29))
  (Utilities|FlowControl|Sequence
    (:then_0
      (if (Variables|Default|GetisKicked)
        (Variables|Default|SetMovement%20prevention true)
        (Components|Movement|StopMovementImmediately (Variables|Character|GetCharacterMovement))
        (Character|LaunchCharacter (+ (* (Math|Vector|GetForwardVector (Transformation|GetWorldRotation (Variables|Collision|GetCapsuleComponent))) -7.5e+02) (* (.z (Math|Vector|GetUpVector (Variables|Collision|GetCapsuleComponent))) 2.5e+02)) false false)
        (Variables|Default|SetisKicked false)
        (Variables|Default|SetisKickedinto true)
        (Utilities|FlowControl|Delay 0.5)
        (Variables|Default|SetisKickedinto false)))
    (:then_1
      (if (Variables|Default|GetMovement%20prevention)
        (Components|Movement|StopMovementImmediately (Variables|Character|GetCharacterMovement))
        (Utilities|FlowControl|Delay 0.3)
        (Variables|Default|SetMovement%20prevention false)
        (else
          (Utilities|FlowControl|Sequence
            (:then_0
              (if (Variables|Default|GetseenPlayer)
                (|MovetoPlayer)
                (elif (Utilities|Array|IsValidIndex (Variables|Default|GetPatrolPointBP) (Variables|Default|GetcurrentNavpoint))
                  (AI|AIMoveTo self "0, 0, 0" (Utilities|Array|Get(acopy) (Variables|Default|GetPatrolPointBP) (Variables|Default|GetcurrentNavpoint)) 5.0 false))))))))))

(event EventDestroyed
  (bind _asbp_top_down_character (Utilities|Casting|CastToBP_TopDownCharacter (Game|Player|GetPlayerPawn 0)))
  (bind _output_get (Variables|/Game/TopDown/Blueprints/BP_TopDownCharacter.BP_TopDownCharacter_C|SetScore _asbp_top_down_character (Variables|/Game/TopDown/Blueprints/BP_TopDownCharacter.BP_TopDownCharacter_C|GetScore _asbp_top_down_character)))
  (bind _result (Math|Integer|IncrementInt _output_get)
    (:%20%20
      (Variables|/Game/TopDown/Blueprints/BP_TopDownCharacter.BP_TopDownCharacter_C|SetScore _asbp_top_down_character _result)
      (Actor|DestroyActor (Variables|Default|GetEnemyRangeFinder)))))

(fn ConstructionScript)